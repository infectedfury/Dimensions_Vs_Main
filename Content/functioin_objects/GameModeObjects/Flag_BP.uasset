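; Capture-the-flag flag actor for side-scroller characters that saves its start location on BeginPlay.
; When not carried, Cube overlap sends the root home for a same-team character, or attaches it to an opposing character's "back" socket and sets Carry.
; While carried, StaticMesh overlap with another team's CapZone detaches the flag, moves StaticMesh (not the root) to the start location and clears Carry, with no scoring here.
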(event OnComponentBeginOverlap(StaticMesh)
  (params (OtherActor :type Actor%20Object%20Reference) (OtherComp :type Primitive%20Component%20Object%20Reference) (OtherBodyIndex :type Integer) (bFromSweep :type Boolean) (SweepResult :type Hit%20Result%20Structure%20%28by%20ref%29))
  (if (Variables|Default|GetCarry)
    (bind _ascap_zone (Utilities|Casting|CastToCapZone OtherActor))
    (if (!= (Variables|/Game/functioin_objects/GameModeObjects/CapZone.CapZone_C|GetTeam _ascap_zone) (Variables|Default|GetTEAM))
      (Class|Actor|DetachRootComponentfromParent false)
      (Transformation|SetWorldLocation (Variables|Default|GetStaticMesh) (Variables|Default|Getstart_location) false false)
      (Variables|Default|SetCarry false))))

(event OnComponentBeginOverlap(Cube)
  (params (OtherActor :type Actor%20Object%20Reference) (OtherComp :type Primitive%20Component%20Object%20Reference) (OtherBodyIndex :type Integer) (bFromSweep :type Boolean) (SweepResult :type Hit%20Result%20Structure%20%28by%20ref%29))
  (if (not (Variables|Default|GetCarry))
    (bind _asside_scroller_character (Utilities|Casting|CastToSideScrollerCharacter OtherActor))
    (if (== (Variables|/Game/characters/SideScrollerCharacter.SideScrollerCharacter_C|GetTeam _asside_scroller_character) (Variables|Default|GetTEAM))
      (Transformation|SetWorldLocation (Variables|Default|GetDefaultSceneRoot) (Variables|Default|Getstart_location) false false)
      (else
        (Class|Actor|AttachRootComponenttoActor self _asside_scroller_character "back" "SnapToTargetIncludingScale" true)
        (Variables|Default|SetCarry true)))))

(event EventBeginPlay
  (Variables|Default|Setstart_location (Transformation|GetWorldLocation (Variables|Default|GetDefaultSceneRoot))))

(fn ConstructionScript)