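; Ball actor that can return its sphere to where it started in the level.
; BeginPlay stores the root component's world location as the start location and prints it.
; Tick polls a reset flag, and when it is set, teleport-free moves the sphere back to that location and clears the flag.
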(event EventTick
  (params (DeltaSeconds :type Float%20%28single-precision%29))
  (if (Variables|Default|Getresetloaction)
    (Transformation|SetWorldLocation (Variables|Default|GetSphere) (stale EventBeginPlay _output_get) false false)
    (Variables|Default|Setresetloaction false)))

(event EventBeginPlay
  (bind _output_get (Variables|Default|Setstart_location (Transformation|GetWorldLocation (Variables|Default|GetDefaultSceneRoot))))
  (Development|PrintString (Utilities|String|ToString(Vector) _output_get)))

(fn ConstructionScript)