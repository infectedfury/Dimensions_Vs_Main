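; Physics ball for a side-scroller game mode that characters can grab, hit, drop and throw, with a flag-triggered reset to its start location.
; Grab overlap disables physics and attaches it to the character's hand socket; active hitbox overlaps knock it away by facing.
; Tick polls the last Collision-overlapping character's flags to detach it for drops, axis-aimed passes or stronger power throws with a dust trail.
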(event OnComponentBeginOverlap(collision)
  (params (OtherActor :type Actor%20Object%20Reference) (OtherComp :type Primitive%20Component%20Object%20Reference) (OtherBodyIndex :type Integer) (bFromSweep :type Boolean) (SweepResult :type Hit%20Result%20Structure%20%28by%20ref%29))
  (bind _sphere (Variables|Default|GetSphere))
  (bind _asside_scroller_character (Utilities|Casting|CastToSideScrollerCharacter OtherActor))
  ;[1 1 1] hitting
  (if (and (Math|Boolean|ORBoolean (and (Variables|/Game/characters/SideScrollerCharacter.SideScrollerCharacter_C|GetHitBoxActive_01 _asside_scroller_character) (== (Variables|/Game/characters/SideScrollerCharacter.SideScrollerCharacter_C|GetHitBox01 _asside_scroller_character) OtherComp)) (and (Variables|/Game/characters/SideScrollerCharacter.SideScrollerCharacter_C|GetHitBoxActive_02 _asside_scroller_character) (== (Variables|/Game/characters/SideScrollerCharacter.SideScrollerCharacter_C|GetHitBox02 _asside_scroller_character) OtherComp)) (and (Variables|/Game/characters/SideScrollerCharacter.SideScrollerCharacter_C|GetHitBoxActive_03 _asside_scroller_character) (== (Variables|/Game/characters/SideScrollerCharacter.SideScrollerCharacter_C|GetHitBox03 _asside_scroller_character) OtherComp))) (not (and (Variables|Default|GetHitDelay) (Variables|Default|GetHeld))))
    (if (Variables|/Game/characters/SideScrollerCharacter.SideScrollerCharacter_C|GetRightFace _asside_scroller_character)
      (Physics|AddImpulse _sphere "0,-10000.000000,10000.000000" "None" false)
      (else
        (Physics|AddImpulse _sphere "0,10000.000000,10000.000000" "None" false)))
    (Variables|Default|SetHitDelay true)
    (Utilities|FlowControl|Delay 0.2)
    (Variables|Default|SetHitDelay false)))

(event OnComponentBeginOverlap(grab_vol)
  (params (OtherActor :type Actor%20Object%20Reference) (OtherComp :type Primitive%20Component%20Object%20Reference) (OtherBodyIndex :type Integer) (bFromSweep :type Boolean) (SweepResult :type Hit%20Result%20Structure%20%28by%20ref%29))
  ;[1 1 1] grabbing ball
  (bind _asside_scroller_character (Utilities|Casting|CastToSideScrollerCharacter OtherActor))
  (if (Math|Boolean|ANDBoolean (not (Variables|Default|GetHeld)) (Variables|/Game/characters/SideScrollerCharacter.SideScrollerCharacter_C|GetGrab_active _asside_scroller_character) (not (Math|Boolean|ANDBoolean (Variables|Default|GetHitDelay) (Variables|Default|GetHeld) (Variables|Default|GetDropBall))))
    (Physics|SetSimulatePhysics (Variables|Default|GetSphere) false)
    (Utilities|FlowControl|Delay 0.1)
    (Class|Actor|AttachRootComponentto (Variables|/Script/Engine.Character|GetMesh _asside_scroller_character) "hand_right" "SnapToTarget" true)
    (Variables|Default|SetHeld true)
    (Variables|/Game/characters/SideScrollerCharacter.SideScrollerCharacter_C|SetBallCary _asside_scroller_character true)
    (Variables|/Game/characters/SideScrollerCharacter.SideScrollerCharacter_C|SetGrab _asside_scroller_character false)
    (Variables|/Game/characters/SideScrollerCharacter.SideScrollerCharacter_C|SetGrab_active _asside_scroller_character false)))

(event Custom|drop
  ;[1 1 1] drop
  (Variables|Default|SetHeld false)
  (Class|SceneComponent|DetachfromParent (Variables|Default|GetSphere) false true)
  (Utilities|FlowControl|Delay 0.01)
  (Physics|SetSimulatePhysics (Variables|Default|GetSphere) true)
  (Development|PrintString "drop" true true "(R=1.000000,G=0.352120,B=0.275569,A=1.000000)")
  (Utilities|FlowControl|Delay 0.2)
  (Variables|Default|SetDropBall false))

(event EventTick
  (params (DeltaSeconds :type Float%20%28single-precision%29))
  (bind _sphere (Variables|Default|GetSphere))
  (Utilities|FlowControl|Sequence
    (:then_0
      ;[1 1 1] Goal
      (if (Variables|Default|Getresetloaction)
        (Class|SceneComponent|DetachfromParent (Variables|Default|GetSphere) false true)
        (Transformation|SetWorldLocation (Variables|Default|GetSphere) (stale EventBeginPlay _output_get) false false)
        (Variables|Default|Setresetloaction false)
        (Physics|SetSimulatePhysics (Variables|Default|GetSphere) false)
        (Utilities|FlowControl|Delay 0.1)
        (Physics|SetSimulatePhysics (Variables|Default|GetSphere) true)
        (Variables|Default|SetHeld false)))
    (:then_1
      (if (Variables|/Game/characters/SideScrollerCharacter.SideScrollerCharacter_C|GetBallDrop (stale OnComponentBeginOverlap(collision) _asside_scroller_character))
        (CallFunction|Drop)))
    (:then_2
      (if (Variables|/Game/characters/SideScrollerCharacter.SideScrollerCharacter_C|GetBallPass (stale OnComponentBeginOverlap(collision) _asside_scroller_character))
        (Variables|Default|SetpassPower (Math|Vector|MakeVector 0.0 (* (Variables|/Game/characters/SideScrollerCharacter.SideScrollerCharacter_C|GetLeftRightAxis (stale OnComponentBeginOverlap(collision) _asside_scroller_character)) -1e+03) (* (Variables|/Game/characters/SideScrollerCharacter.SideScrollerCharacter_C|GetUpDownAxis (stale OnComponentBeginOverlap(collision) _asside_scroller_character)) 1e+03)))
        (Variables|Default|SetHeld false)
        (Class|SceneComponent|DetachfromParent (Variables|Default|GetSphere) false true)
        (Utilities|FlowControl|Delay 0.01)
        (Physics|SetSimulatePhysics (Variables|Default|GetSphere) true)
        (Utilities|FlowControl|Delay 0.01)
        (Physics|AddImpulse (Variables|Default|GetSphere) (Variables|Default|GetpassPower) "None" false)
        (Development|PrintString "throw" true true "(R=1.000000,G=0.352120,B=0.275569,A=1.000000)")
        (Utilities|FlowControl|Delay 0.2)
        (Variables|Default|SetThrowBall_01 false)))
    (:then_3
      (if (Variables|/Game/characters/SideScrollerCharacter.SideScrollerCharacter_C|GetBallPower (stale OnComponentBeginOverlap(collision) _asside_scroller_character))
        (Variables|Default|SetpassPower (Math|Vector|MakeVector 0.0 (* (Variables|/Game/characters/SideScrollerCharacter.SideScrollerCharacter_C|GetLeftRightAxis (stale OnComponentBeginOverlap(collision) _asside_scroller_character)) -2e+03) (* (Variables|/Game/characters/SideScrollerCharacter.SideScrollerCharacter_C|GetUpDownAxis (stale OnComponentBeginOverlap(collision) _asside_scroller_character)) 2e+03)))
        (Variables|Default|SetHeld false)
        (Class|SceneComponent|DetachfromParent (Variables|Default|GetSphere) false true)
        (Utilities|FlowControl|Delay 0.01)
        (Effects|SpawnEmitterAttached "/Game/Particle/Emitters/Smashed_DustTrail_Omnidirectional.Smashed_DustTrail_Omnidirectional" _sphere "None" "0, 0, 0" "0, 0, 0" "KeepRelativeOffset" false)
        (Physics|SetSimulatePhysics _sphere true)
        (Utilities|FlowControl|Delay 0.01)
        (Physics|AddImpulse (Variables|Default|GetSphere) (Variables|Default|GetpassPower) "None" false)
        (Development|PrintString "power" true true "(R=1.000000,G=0.352120,B=0.275569,A=1.000000)")
        (Utilities|FlowControl|Delay 0.5)
        (Variables|Default|SetThrowBall_02 false)))))

(event EventBeginPlay
  ;[1 1 1] init
  (bind _output_get (Variables|Default|SetstartLocation (Transformation|GetWorldLocation (Variables|Default|GetSphere))))
  (Development|PrintString (Utilities|String|ToString(Vector) _output_get)))

(fn ConstructionScript)